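; BP_Enemy is an AI enemy that wanders the NavMesh, pursues the player, and deals contact damage.
; Tick issues delayed moves to random nearby reachable points until PawnSensing sees any pawn, setting CanSee and triggering a move toward the player.
; CanSee stays true afterward, as the retriggerable-delay reset sits in unconnected nodes.
; Incoming damage reduces Health and destroys the actor at zero, while capsule overlap applies fixed damage to the other actor.
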(event OnSeePawn(PawnSensing)
  (params (Pawn :type Pawn%20Object%20Reference))
  ;[1 1 1] 네비메쉬를 이용한 적 AI
  (Variables|Default|SetCanSee true)
  (CallFunction|FollowPlayer))

(event OnComponentBeginOverlap(Capsule)
  (params (OverlappedComponent :type Primitive%20Component%20Object%20Reference) (OtherActor :type Actor%20Object%20Reference) (OtherComp :type Primitive%20Component%20Object%20Reference) (OtherBodyIndex :type Integer) (bFromSweep :type Boolean) (SweepResult :type Hit%20Result%20Structure%20%28by%20ref%29))
  ;[1 1 1] 적에게 닿으면 데미지를 입힘
  (Game|Damage|ApplyDamage OtherActor 1e+01 0 self))

(event Custom|Follow_Player
  ;[1 1 1] 네비메쉬를 이용한 적 AI
  (if (Variables|Default|GetCanSee)
    (AI|AIMoveTo self "0, 0, 0" (Game|GetPlayerCharacter 0) 5.0 false)))

(event EventTick
  (params (DeltaSeconds :type Float%20%28single-precision%29))
  ;[1 1 1] 네비메쉬를 이용한 적 AI
  (if (not (Variables|Default|GetCanSee))
    (Utilities|FlowControl|Delay (Math|Random|RandomFloatinRange 2.0 5.0))
    (AI|AIMoveTo self (.RandomLocation (AI|Navigation|GetRandomReachablePointinRadius (Transformation|GetActorLocation) 5e+02 0 0)) 0 5.0 false)))

(event Game|Damage|EventAnyDamage
  (params (Damage :type Float%20%28single-precision%29) (DamageType :type Damage%20Type%20Object%20Reference) (InstigatedBy :type Controller%20Object%20Reference) (DamageCauser :type Actor%20Object%20Reference))
  ;[1 1 1] 피해를 입으면 체력이 닳고 체력이 0이 되면 사라짐
  (bind _output_get (Variables|Default|SetHealth (- (Variables|Default|GetHealth) Damage)))
  (if (<= _output_get 0.0)
    (Actor|DestroyActor)))

(fn ConstructionScript)